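; BP_Cup is a timed tea order actor that scores the ingredients added to it.
; Construction shuffles the tea ingredient list and keeps up to five as needed; BeginPlay starts a looping countdown and pushes needed ingredients to a widget.
; AddIngridientToCup rejects duplicates, updates the recipe widget and prices the cup by matching ingredients.
; Five ingredients or timer expiry calls FinishCup, which dispatches position, price and correctness, then destroys the actor.
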(event `self.ReceiveBeginPlay`
  ;[1 1 1] BeginPlay
  (set `self.Current Time Remaining` (`self.Expected Timer Duration`))
  (bind _returnvalue (`KismetSystemLibrary.K2_SetTimerDelegate` (`|CreateDelegate` :!event `SetValueOnTimer`) (`self.Timer Tick Duration`) true true))
  (set `self.Timer Reference` _returnvalue)
  (`KismetSystemLibrary.Delay` 1.0)
  (for _array_element (`self.neededIngredients`)
    (`KismetSystemLibrary.Delay` 5.0)
    (bind _asw_show_needed_ingredient (cast `/Game/W_ShowNeededIngredient` (`WidgetComponent.GetWidget` (`self.NeededIngredient`))))
    (set `/Game/W_ShowNeededIngredient.TextBlock` (`KismetTextLibrary.Conv_StringToText` _array_element) _asw_show_needed_ingredient)))

(event `SetValueOnTimer`
  ;[1 1 1] TimerFunction
  (bind _output_get (set `self.Current Time Remaining` (- (`self.Current Time Remaining`) (`self.Timer Tick Duration`))))
  (bind _asw_cup_timer (cast `/Game/UI/W_CupTimer` (`WidgetComponent.GetWidget` (`self.TimeLeftWidget`))))
  (set `/Game/UI/W_CupTimer.TextBlock` (`KismetTextLibrary.Conv_DoubleToText` (`KismetMathLibrary.Conv_Int64ToDouble` (`KismetMathLibrary.Round64` _output_get)) "HalfToEven") _asw_cup_timer)
  (if (<= _output_get 0.2)
    (`self.FinishCup`)))

(fn `AddIngridientToCup`
  (params (ingridient :type String))
  (bind _ingredientsincuparray (`self.IngredientsInCupArray`))
  (bind _returnvalue (`KismetArrayLibrary.Array_Contains` (`self.neededIngredients`) ingridient))
  (if (`KismetArrayLibrary.Array_Contains` _ingredientsincuparray ingridient)
    (`KismetSystemLibrary.PrintString` "Ingridient already in cup")
    (else
      (`KismetArrayLibrary.Array_Add` _ingredientsincuparray ingridient)
      (if _returnvalue
        (set `self.ingredientBalance` (+ (`self.ingredientBalance`) 1)))
      (bind _asw_cup_frame (cast `/Game/UI/W_CupFrame` (`WidgetComponent.GetWidget` (`self.ReciptWidget1`))))
      (`/Game/UI/W_CupFrame.AddText` _asw_cup_frame _returnvalue ingridient)
      (`self.CalculateRecipt`)
      ; Max Ingredience in Cup
      (if (== (`KismetArrayLibrary.Array_Length` (`self.IngredientsInCupArray`)) 5)
        (`self.FinishCup`)))))

(fn `CalculateRecipt`
  (bind _returnvalue (* (`self.ingredientBalance`) 3))
  (bind _asw_cup_frame (cast `/Game/UI/W_CupFrame` (`WidgetComponent.GetWidget` (`self.ReciptWidget1`))))
  (`/Game/UI/W_CupFrame.SetPrice` _asw_cup_frame (`KismetStringLibrary.Conv_IntToString` _returnvalue))
  (set `self.price` _returnvalue))

(fn `FinishCup`
  (`self.NewEventDispatcher` (`self.positionId`) (`self.price`) (> (`self.ingredientBalance`) 0))
  (`self.K2_DestroyActor`))

(fn `UserConstructionScript`
  (bind _idcounter (`self.idCounter`))
  (bind _neededingredients (`self.neededIngredients`))
  (set `self.id` (+ (`self.id`) _idcounter))
  (set `self.idCounter` (+ _idcounter 1))
  (bind _output_get (set `self.neededIngredients` (`self.teaIngredientArray`)))
  (`KismetArrayLibrary.Array_Shuffle` _output_get)
  (while (> (`KismetArrayLibrary.Array_Length` _output_get) 5)
    (set `self.neededIngredients` _neededingredients)
    (`KismetArrayLibrary.Array_Remove` _neededingredients (`KismetArrayLibrary.Array_LastIndex` _neededingredients)))
  (for _array_element _neededingredients
    (`KismetSystemLibrary.PrintString` _array_element)))